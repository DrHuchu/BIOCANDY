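; Enemy character Blueprint for a variant that starts prone and begins moving once it senses the player.
; BeginPlay sets both the EnemyFsm state and the ABP_Enemy1 anim state to Prone; pawn sight of Player_Jill or any perception update switches both to Move unless dead, attacking or shocked.
; Shock, burn and damage events play montages, while RandomRoam walks to a random nearby reachable point, then returns to Idle.
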(event OnSeePawn(pawnSensor)
  (params (Pawn :type Pawn%20Object%20Reference))
  (if (not (Utilities|Enum|Equal(Enum) (Variables|/Script/BIOCANDY.EnemyFSM|GetmState (Variables|Default|GetenemyFsm)) "Die"))
    (if (not (Utilities|Enum|Equal(Enum) (Variables|/Script/BIOCANDY.EnemyFSM|GetmState (Variables|Default|GetenemyFsm)) "Attack"))
      (if (not (Utilities|Enum|Equal(Enum) (Variables|/Script/BIOCANDY.EnemyFSM|GetmState (Variables|Default|GetenemyFsm)) "Shocked"))
        (Utilities|Casting|CastToPlayer_Jill Pawn)
        (Variables|/Script/BIOCANDY.EnemyFSM|SetmState (Variables|Default|GetenemyFsm) "Move")
        (bind _asabp_enemy_1 (Utilities|Casting|CastToABP_Enemy1 (Components|SkeletalMesh|GetAnimInstance (Variables|Character|GetMesh))))
        (Variables|/Script/BIOCANDY.EnemyAnim|Setstate _asabp_enemy_1 "Move")))))

(event OnPerceptionUpdated(AIPerception)
  (params (UpdatedActors :type Array%20of%20Actor%20Object%20References))
  (if (not (Utilities|Enum|Equal(Enum) (Variables|/Script/BIOCANDY.EnemyFSM|GetmState (Variables|Default|GetenemyFsm)) "Die"))
    (if (not (Utilities|Enum|Equal(Enum) (Variables|/Script/BIOCANDY.EnemyFSM|GetmState (Variables|Default|GetenemyFsm)) "Attack"))
      (if (not (Utilities|Enum|Equal(Enum) (Variables|/Script/BIOCANDY.EnemyFSM|GetmState (Variables|Default|GetenemyFsm)) "Shocked"))
        (Variables|/Script/BIOCANDY.EnemyFSM|SetmState (Variables|Default|GetenemyFsm) "Move")
        (bind _asabp_enemy_1 (Utilities|Casting|CastToABP_Enemy1 (Components|SkeletalMesh|GetAnimInstance (Variables|Character|GetMesh))))
        (Variables|/Script/BIOCANDY.EnemyAnim|Setstate _asabp_enemy_1 "Move")))))

(event EventBeginPlay
  (Variables|/Script/BIOCANDY.EnemyFSM|SetmState (Variables|Default|GetenemyFsm) "Prone")
  (bind _asabp_enemy_1 (Utilities|Casting|CastToABP_Enemy1 (Components|SkeletalMesh|GetAnimInstance (Variables|Character|GetMesh self))))
  (Variables|/Script/BIOCANDY.EnemyAnim|Setstate _asabp_enemy_1 "Prone"))

(event Collision|EventActorBeginOverlap
  (params (OtherActor :type Actor%20Object%20Reference)))

(event EventRandomRoam
  (bind _self self)
  (AI|AIMoveTo _self (.RandomLocation (AI|Navigation|GetRandomReachablePointinRadius (Transformation|GetActorLocation) (Math|Random|RandomFloatinRange 2e+02 5e+02) 0 0)) 0 5.0 false
    (:OnSuccess
      (AI|Navigation|StopMovement (AI|GetAIController _self))
      (Variables|/Script/BIOCANDY.EnemyFSM|SetmState (Variables|Default|GetenemyFsm) "Idle")
      (bind _asabp_enemy_1 (Utilities|Casting|CastToABP_Enemy1 (Components|SkeletalMesh|GetAnimInstance (Variables|Character|GetMesh))))
      (Variables|/Script/BIOCANDY.EnemyAnim|Setstate _asabp_enemy_1 "Idle")
      (Variables|Default|SetbRoamEnd false))))

(event EventOnMyDamage
  (params (sectionName :type Name :default "None"))
  (Animation|PlayAnimMontage "/Game/BluePrint/EnemyAnimMontage_Damage+Die.EnemyAnimMontage_Damage+Die" 1.0 sectionName))

(event EventOnMyBurn
  (Animation|PlayAnimMontage "/Game/Mixamo/WarZombie/mixamoconverter/Mixamo_Anim/EnemyAnimMontage_Burnt.EnemyAnimMontage_Burnt" 1.0 "None"))

(event EventOnMyShock
  (Animation|PlayAnimMontage "/Game/Mixamo/WarZombie/mixamoconverter/Mixamo_Anim/EnemyAnimMontage_Electrocuted.EnemyAnimMontage_Electrocuted" 1.0 "None"))

(event EventTick
  (params (DeltaSeconds :type Float%20%28single-precision%29)))

(fn ConstructionScript)