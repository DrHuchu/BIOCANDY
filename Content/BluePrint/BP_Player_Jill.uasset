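; Player character Blueprint for Jill, a pistol shooter with zoom aiming and selectable outfits.
; Right mouse toggles the AnimBP zoom flag; firing spends ammo and line-traces from the camera, calling reload when the magazine is empty.
; Hit physical surfaces select head or body damage through the enemy's FSM, explodable barrel and generator reactions, and impact particles.
; The construction script applies OutfitID by showing ranges of mesh material sections.
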(event EventBeginPlay
  (Transformation|AttachComponentToComponent (Variables|Default|GetgunMeshComp) (Variables|Character|GetMesh) "PistolSocket2" "SnapToTarget" "KeepRelative" "KeepRelative" true))

(event Collision|EventActorBeginOverlap
  (params (OtherActor :type Actor%20Object%20Reference)))

(event Input|ActionEvents|InputActionFire
  (params (Key :type Key%20Structure :default "None"))
  (bind _magui (Variables|Default|GetmagUI))
  (bind _cameracomp (Variables|Default|GetcameraComp))
  (bind _returnvalue (Transformation|GetWorldLocation _cameracomp))
  (:Pressed
    (if (Variables|Default|GetIsShootReady)
      (if (> (Variables|Default|GetpistolCountMag) 0)
        (Variables|Default|SetpistolCountMag (- (Variables|Default|GetpistolCountMag) 1))
        (Widget|RemovefromParent _magui)
        (UserInterface|Viewport|AddtoViewport _magui 0)
        (bind (_outhit _returnvalue_2) (Collision|LineTraceByChannel _returnvalue (+ _returnvalue (* (Math|Vector|GetForwardVector (Transformation|GetWorldRotation _cameracomp)) 1e+05)) "TraceTypeQuery1" false 0 "None"))
        (if _returnvalue_2
          (Variables|Default|SetNormal (.Normal (Collision|BreakHitResult _outhit)))
          (Variables|Default|SetImpact%20Point (.ImpactPoint (Collision|BreakHitResult _outhit)))
          (Variables|Default|SetHit%20Actor (.HitActor (Collision|BreakHitResult _outhit)))
          (switch Utilities|FlowControl|Switch|SwitchonEPhysicalSurface (Variables|/Script/PhysicsCore.PhysicalMaterial|GetSurfaceType (.PhysMat (Collision|BreakHitResult _outhit)))
            (:SurfaceType_Default
              (Development|PrintString "default"))
            (:SurfaceType1
              ;[1 1 1] 좀비 피격
              (Development|PrintString "head")
              (CallFunction|DamageHead)
              (Effects|SpawnEmitteratLocation "/Game/Realistic_Starter_VFX_Pack_Vol2/Particles/Blood/P_Blood_Splat_Cone.P_Blood_Splat_Cone" (Variables|Default|GetImpact%20Point) (Math|Conversions|RotationFromXVector (Variables|Default|GetNormal)) :!label _label))
            (:SurfaceType2
              (Development|PrintString "body")
              (CallFunction|DamageBody :!label _label_2)
              (goto _label))
            (:SurfaceType3
              (Development|PrintString "arm")
              (goto _label_2))
            (:SurfaceType4
              (Development|PrintString "leg")
              (goto _label_2))
            (:SurfaceType5
              ;[1 1 1] 드럼통 폭발
              (bind _asexplodable (Utilities|Casting|CastToExplodable (Variables|Default|GetHit%20Actor)))
              (Class|Explodable|Explosion _asexplodable)
              (Effects|SpawnEmitteratLocation "/Game/Realistic_Starter_VFX_Pack_Vol2/Particles/Destruction/P_Destruction_Metal.P_Destruction_Metal" (Variables|Default|GetImpact%20Point) (Math|Conversions|RotationFromXVector (Variables|Default|GetNormal))))
            (:SurfaceType6
              ;[1 1 1] 발전기 폭발
              (bind _asexplodable_2 (Utilities|Casting|CastToExplodable (Variables|Default|GetHit%20Actor)))
              (Class|Explodable|ElectricShock _asexplodable_2)
              (Effects|SpawnEmitteratLocation "/Game/Realistic_Starter_VFX_Pack_Vol2/Particles/Destruction/P_Destruction_Metal.P_Destruction_Metal" (Variables|Default|GetImpact%20Point) (Math|Conversions|RotationFromXVector (Variables|Default|GetNormal))))
            (:SurfaceType7
              ;[1 1 1] 아스팔트
              (Effects|SpawnEmitteratLocation "/Game/Realistic_Starter_VFX_Pack_Vol2/Particles/Hit/P_Asphalt_small.P_Asphalt_small" (Variables|Default|GetImpact%20Point)))
            (:SurfaceType8
              ;[1 1 1] 메탈
              (Effects|SpawnEmitteratLocation "/Game/Realistic_Starter_VFX_Pack_Vol2/Particles/Destruction/P_Destruction_Metal.P_Destruction_Metal" (Variables|Default|GetImpact%20Point) (Math|Conversions|RotationFromXVector (Variables|Default|GetNormal))))
            (:SurfaceType9
              ;[1 1 1] 나무
              (Effects|SpawnEmitteratLocation "/Game/Realistic_Starter_VFX_Pack_Vol2/Particles/Hit/P_Wood.P_Wood" (Variables|Default|GetImpact%20Point) (Math|Conversions|RotationFromXVector (Variables|Default|GetNormal))))))
        (elif (> (Variables|Default|GetpistolCountBag) 0)
          (Class|PlayerJill|OnActionReload))))))

(event Input|MouseEvents|RightMouseButton
  (params (Key :type Key%20Structure :default "None"))
  ;[1 1 1] 우클릭 조준
  (:Pressed
    (bind _asabp_player_jill (Utilities|Casting|CastToABP_PlayerJill (Components|SkeletalMesh|GetAnimInstance (Variables|Character|GetMesh))))
    (Variables|/Game/Animaiton/ABP_PlayerJill.ABP_PlayerJill_C|SetIszoomin _asabp_player_jill true))
  (:Released
    (bind _asabp_player_jill_2 (Utilities|Casting|CastToABP_PlayerJill (Components|SkeletalMesh|GetAnimInstance (Variables|Character|GetMesh))))
    (Variables|/Game/Animaiton/ABP_PlayerJill.ABP_PlayerJill_C|SetIszoomin _asabp_player_jill_2 false)))

(fn ConstructionScript
  (CallFunction|SetOutfit (Variables|Default|GetOutfit%20ID)))

(fn SetOutfit
  (params (outfit%20ID :type Integer))
  (Class|SkinnedMeshComponent|ShowAllMaterialSections (Variables|Character|GetMesh))
  (for _index (range 20 76)
    (Class|SkinnedMeshComponent|ShowMaterialSection (Variables|Character|GetMesh) _index 0 false)
    (switch int outfit%20ID
      (:1
        (for _index_2 (range 20 31)
          (Class|SkinnedMeshComponent|ShowMaterialSection (Variables|Character|GetMesh) _index_2 0 true)))
      (:2
        (for _index_3 (range 32 46)
          (Class|SkinnedMeshComponent|ShowMaterialSection (Variables|Character|GetMesh) _index_3 0 true)))
      (:3
        (for _index_4 (range 47 50)
          (Class|SkinnedMeshComponent|ShowMaterialSection (Variables|Character|GetMesh) _index_4 0 true)))
      (:4
        (for _index_5 (range 51 54)
          (Class|SkinnedMeshComponent|ShowMaterialSection (Variables|Character|GetMesh) _index_5 0 true)))
      (:5
        (for _index_6 (range 55 58)
          (Class|SkinnedMeshComponent|ShowMaterialSection (Variables|Character|GetMesh) _index_6 0 true)
          (for _index_7 (range 33 46)
            (Class|SkinnedMeshComponent|ShowMaterialSection (Variables|Character|GetMesh) _index_7 0 true))))
      (:6
        (for _index_8 (range 59 76)
          (Class|SkinnedMeshComponent|ShowMaterialSection (Variables|Character|GetMesh) _index_8 0 true))))))

(fn DamageHead
  (bind _asenemy (Utilities|Casting|CastToEnemy (Variables|Default|GetHit%20Actor)))
  (Class|EnemyFSM|OnDamageProcess (Variables|/Script/BIOCANDY.Enemy|GetenemyFsm _asenemy) 10))

(fn DamageBody
  (bind _asenemy (Utilities|Casting|CastToEnemy (Variables|Default|GetHit%20Actor)))
  (Class|EnemyFSM|OnDamageProcess (Variables|/Script/BIOCANDY.Enemy|GetenemyFsm _asenemy) 3))