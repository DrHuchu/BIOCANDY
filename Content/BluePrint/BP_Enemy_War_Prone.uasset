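; BP_Enemy_War_Prone is an enemy Blueprint variant that starts in the Prone state.
; On BeginPlay it sets the EnemyFsm state to Prone, then casts the mesh's anim instance to ABP_Enemy1 and sets its State to match.
; The graph adds no other active logic, as the overlap and tick events are disabled and the construction script only calls the parent.
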(event EventBeginPlay
  (Variables|/Script/BIOCANDY.EnemyFSM|SetmState (Variables|Default|GetenemyFsm) "Prone")
  (bind _asabp_enemy_1 (Utilities|Casting|CastToABP_Enemy1 (Components|SkeletalMesh|GetAnimInstance (Variables|Character|GetMesh self))))
  (Variables|/Script/BIOCANDY.EnemyAnim|Setstate _asabp_enemy_1 "Prone"))

(event Collision|EventActorBeginOverlap
  (params (OtherActor :type Actor%20Object%20Reference))
  (|CallParentFunction OtherActor) ; This node is disabled and will not be called.\nDrag off pins to build functionality.
)

(event EventTick
  (params (DeltaSeconds :type Float%20%28single-precision%29))
  (|CallParentFunction DeltaSeconds) ; This node is disabled and will not be called.\nDrag off pins to build functionality.
)

(fn ConstructionScript
  (|CallParentFunction))